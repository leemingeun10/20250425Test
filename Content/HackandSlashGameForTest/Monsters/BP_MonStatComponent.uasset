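; Monster stat component that holds a monster's data-table stats and current HP in the hack-and-slash game.
; InitializeMonstat loads a row from DT_Monster and starts current HP at MaxHP, and AddDamage subtracts damage from it without clamping.
; Looping 0.05-second timers from BeginPlay poll these stats, pushing name and HP ratio to the owning BP_BaseMonster's name tag widget.
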(event EventBeginPlay
  (Utilities|Time|SetTimerbyFunctionName 0 "UpdateName" 0.05 true)
  (Utilities|Time|SetTimerbyFunctionName 0 "UpdateHP" 0.05 true))

(event EventTick
  (params (DeltaSeconds :type Float%20%28single-precision%29)))

(fn InitializeMonstat
  (params (RowName :type Name))
  (bind _returnvalue (Utilities|GetDataTableRow "/Game/HackandSlashGameForTest/Monsters/DT_Monster.DT_Monster" RowName)
    (:then
      (Variables|Default|SetMonStat (Utilities|Struct|MakeST_CurMonStat _returnvalue (.MaxHP (Utilities|Struct|BreakST_Monster _returnvalue)))))))

(fn UpdateHP
  (bind _monstat (Variables|Default|GetMonStat))
  (bind _asbp_base_monster (Utilities|Casting|CastToBP_BaseMonster (Components|GetOwner)))
  (Default|UpdateHP (Variables|/Game/HackandSlashGameForTest/Character/BP_NameTagComponet.BP_NameTagComponet_C|GetNameTagWidget (Variables|/Game/HackandSlashGameForTest/Monsters/BP_BaseMonster.BP_BaseMonster_C|GetBP_NameTagComponet _asbp_base_monster)) (/ (.curhp _monstat) (.maxhp (.monstat _monstat)))))

(fn UpdateName
  (bind _asbp_base_monster (Utilities|Casting|CastToBP_BaseMonster (Components|GetOwner)))
  (Default|UpDateName (Variables|/Game/HackandSlashGameForTest/Character/BP_NameTagComponet.BP_NameTagComponet_C|GetNameTagWidget (Variables|/Game/HackandSlashGameForTest/Monsters/BP_BaseMonster.BP_BaseMonster_C|GetBP_NameTagComponet _asbp_base_monster)) (Utilities|String|ToString(Name) (.name (.monstat (Variables|Default|GetMonStat))))))

(fn AddDamage
  (params (damage :type Float%20%28double-precision%29))
  (Utilities|Struct|SetmembersinST_CurMonStat (Variables|Default|GetMonStat) (- (.curhp (Variables|Default|GetMonStat)) damage)))