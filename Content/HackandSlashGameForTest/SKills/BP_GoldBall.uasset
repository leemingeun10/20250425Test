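; BP_GoldBall is a skill projectile that damages what it passes and destroys itself five seconds after spawning.
; Each Tick moves the FireBall component forward by a fixed step, without sweep or delta-time scaling, so speed depends on frame rate.
; A Tick-accumulated timer periodically applies small-radius radial damage at the ball's location, ignoring the player pawn and crediting the player controller.
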(event EventBeginPlay
  (Utilities|FlowControl|Delay 5.0)
  (Actor|DestroyActor))

(event Collision|EventActorBeginOverlap
  (params (OtherActor :type Actor%20Object%20Reference)))

(event EventTick
  (params (DeltaSeconds :type Float%20%28single-precision%29))
  (Utilities|FlowControl|Sequence
    (:then_0
      (bind _output_get (Variables|Default|Settimer (+ DeltaSeconds (Variables|Default|Gettimer))))
      (if (> _output_get 0.1)
        (Variables|Default|Settimer 0.0)
        (Game|Damage|ApplyRadialDamage 2e+01 (Transformation|GetWorldLocation (Variables|Default|GetFireBall)) 5e+01 0 (Utilities|Array|MakeArray (Game|Player|GetPlayerPawn 0)) self (Game|GetPlayerController 0) false "ECC_Visibility")))
    (:then_1
      (CallFunction|ShootBall))))

(fn ConstructionScript)

(fn ShootBall
  (Transformation|AddWorldOffset (Variables|Default|GetFireBall) (* (Math|Vector|GetForwardVector (Variables|Default|GetFireBall)) 5e+01) false false))