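; Spawner component that repeatedly creates random monsters around its owning actor.
; A looping timer started on BeginPlay calls SpawnMonster every second.
; Each call picks a random DT_Monster row and spawns its MonsterClass with AI at a random navigable point within a fixed radius of the owner.
; The row name is then passed to BP_BaseMonster to initialize the monster's stats.
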(event EventBeginPlay
  (Utilities|Time|SetTimerbyFunctionName 0 "SpawnMonster" 1.0 true))

(event EventTick
  (params (DeltaSeconds :type Float%20%28single-precision%29)))

(fn SpawnMonster
  (bind _outrownames (DataTable|GetDataTableRowNames "/Game/HackandSlashGameForTest/Monsters/DT_Monster.DT_Monster"))
  (bind _output_get (Variables|Default|SetRowName (.OutItem (Utilities|Array|Random _outrownames))))
  (bind _returnvalue (Utilities|GetDataTableRow "/Game/HackandSlashGameForTest/Monsters/DT_Monster.DT_Monster" _output_get)
    (:then
      (bind _randomlocation (Class|NavigationSystemV1|GetRandomLocationinNavigableRadius (Transformation|GetActorLocation (Components|GetOwner)) 1e+03 0 0))
      (bind _returnvalue_2 (AI|SpawnAIFromClass (.MonsterClass (Utilities|Struct|BreakST_Monster _returnvalue)) 0 _randomlocation "0, 0, 0" false 0))
      (bind _asbp_base_monster (Utilities|Casting|CastToBP_BaseMonster _returnvalue_2))
      (Default|InitalizeMonStat _asbp_base_monster (Variables|Default|GetRowName)))))